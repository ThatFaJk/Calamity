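; Spline placement actor that fills its spline with randomly alternated instances of two configurable meshes, built in the Construction Script.
; A loop picks one of two instanced mesh components per step and advances by that mesh's X bounds plus an offset until the spline length is reached.
; Instances follow spline location and rotation, with random local Y, roll and yaw offsets.
; GetLocationAtIndex and its Spacing-based logic are unused leftovers.
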(fn `GetLocationAtIndex`
  (params (A :type "Float (double-precision)"))
  (returns (ReturnValue :type "Vector Structure"))
  (return (`SplineComponent.GetLocationAtDistanceAlongSpline` (`self.Spline`) (* A (`self.Spacing`)) "Local")))

(fn `UserConstructionScript`
  (locals (NumberOfInstances :type Integer :default 0))
  (bind (_returnvalue_x _returnvalue_y _returnvalue_z) (`KismetMathLibrary.BreakVector` (`SplineComponent.GetLocationAtDistanceAlongSpline` (`self.Spline`) (- (`self.totalSpacing`) (`self.HalfExtent`)) "Local")))
  (bind (_returnvalue_roll _returnvalue_pitch _returnvalue_yaw) (`KismetMathLibrary.BreakRotator` (`SplineComponent.GetRotationAtDistanceAlongSpline` (`self.Spline`) (- (`self.totalSpacing`) (`self.HalfExtent`)) "Local")))
  (`StaticMeshComponent.SetStaticMesh` (`self.InstancedStaticMesh`) (`self.Mesh`))
  (`StaticMeshComponent.SetStaticMesh` (`self.InstancedStaticMesh1`) (`self.Mesh2`))
  (set `self.totalSpacing` 0.0)
  (while (> (`SplineComponent.GetSplineLength` (`self.Spline`)) (`self.totalSpacing`))
    (bind _output_get (set `self.CurrentMesh` (select `int` (`KismetMathLibrary.RandomIntegerInRange` 0 1) :`0` (`self.InstancedStaticMesh`) :`1` (`self.InstancedStaticMesh1`))))
    (bind _returnvalue (`StaticMesh.GetBounds` (`StaticMeshComponent.StaticMesh` _output_get)))
    (set `self.HalfExtent` (.x (`.BoxExtent` (`KismetMathLibrary.BreakBoxSphereBounds` _returnvalue))))
    (set `self.totalSpacing` (+ (+ (* (.x (`.BoxExtent` (`KismetMathLibrary.BreakBoxSphereBounds` _returnvalue))) 2.0) (`self.Offset`)) (`self.totalSpacing`)))
    (if (> (`SplineComponent.GetSplineLength` (`self.Spline`)) (`self.totalSpacing`))
      (`InstancedStaticMeshComponent.AddInstance` _output_get (`KismetMathLibrary.MakeTransform` (`KismetMathLibrary.MakeVector` _returnvalue_x (+ _returnvalue_y (`KismetMathLibrary.RandomFloatInRange` (`self.RandomYOffsetMin`) (`self.RandomYOffsetMax`))) _returnvalue_z) (`KismetMathLibrary.MakeRotator` (+ (`KismetMathLibrary.RandomFloatInRange` (`self.RandomUpRotationOffsetMin`) (`self.RandomUpRotationOffsetMax`)) _returnvalue_roll) _returnvalue_pitch (+ _returnvalue_yaw (`KismetMathLibrary.RandomFloatInRange` (`self.RandomSideRotationOffsetMin`) (`self.RandomSideRotationOffsetMax`))))) false))))