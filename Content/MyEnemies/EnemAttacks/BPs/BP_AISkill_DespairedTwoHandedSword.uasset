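; One-shot AI skill actor for the Despaired two-handed sword attack, dealing melee damage in front of its owning pawn.
; On BeginPlay the server runs a multi sphere trace forward from the owner and passes the hits to DamageMultipleEnemies with the skill's damage and effects.
; It then has the owner multicast a weapon swoosh sound, at the first hit if damage landed, otherwise at the skill actor.
; The actor destroys itself immediately afterwards.
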(event `self.ReceiveBeginPlay`
  (bind _pawnowner (`self.PawnOwner`))
  (bind _returnvalue (+ (`self.K2_GetActorLocation` _pawnowner) (* (`self.GetActorForwardVector` _pawnowner) 70.0)))
  ;[0.03125 0.03125 0.03125] Deal damage using a sphere trace
  (`parent.ReceiveBeginPlay`)
  (`|ExecutionSequence`
    (:`then_0`
      (`/Engine/EditorBlueprintResources/ActorMacros.Switch Has Authority`
        (:`Authority`
          (bind (_outhits _returnvalue_2) (`KismetSystemLibrary.SphereTraceMultiForObjects` _returnvalue (+ _returnvalue (* (`self.GetActorForwardVector` (`self.PawnOwner`)) 130.0)) 60.0 (`|MakeArray` "ObjectTypeQuery3" "ObjectTypeQuery2" :!type "EObjectTypeQuery Enum") false (`|MakeArray` (`self.PawnOwner`) :!type "Actor Object Reference")))
          (if _returnvalue_2
            (bind _hitenemies (`self.DamageMultipleEnemies` _outhits (`self.SkillDamage`) (`self.DamageType`) true))
            (if (`KismetArrayLibrary.Array_IsValidIndex` _hitenemies)
              (bind _pawnowner_2 (`self.PawnOwner`)
                (:`then`
                  (message `/Game/ActionRPGStarterSystem/Skills/Blueprint/SkillComponent/IT_SkillEffects.Skill_MCSound` _pawnowner_2 "/Game/MySounds/Weapons/WeaponSwooshMetaSound.WeaponSwooshMetaSound" (`.Location` (`GameplayStatics.BreakHitResult` (`|GetArrayItem` _outhits)))))
                (:`else`))
              (else
                (bind _pawnowner_3 (`self.PawnOwner` :!label _label)
                  (:`then`
                    (message `/Game/ActionRPGStarterSystem/Skills/Blueprint/SkillComponent/IT_SkillEffects.Skill_MCSound` _pawnowner_3 "/Game/MySounds/Weapons/WeaponSwooshMetaSound.WeaponSwooshMetaSound" (`self.K2_GetActorLocation`)))
                  (:`else`))))
            (else
              (goto _label))))))
    (:`then_1`
      (`self.K2_DestroyActor`))))

(fn `UserConstructionScript`
  (`parent.UserConstructionScript`))