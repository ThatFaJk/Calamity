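; AI home actor that spawns a set of AI on the server when the player enters its box and despawns them on exit.
; Spawns use random points within Radius, validated by floor and capsule traces, or a saved transform for stationary AI.
; Destroyed AI can return through a delayed BP_AIRespawner that calls back into the home.
; New spawns inherit aggro targets from living members and can be linked as a party.
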(event `self.ReceiveTick`
  (params (DeltaSeconds :type "Float (single-precision)"))
  ;[1 1 1] debug
)

(event `self.ReceiveBeginPlay`)

(event `self.Box.OnComponentBeginOverlap`
  (params (OverlappedComponent :type "PrimitiveComponent Object Reference") (OtherActor :type "Actor Object Reference") (OtherComp :type "PrimitiveComponent Object Reference") (OtherBodyIndex :type Integer) (bFromSweep :type Boolean) (SweepResult :type "HitResult Structure (by ref)"))
  (if (== OtherActor (`GameplayStatics.GetPlayerCharacter` 0))
    ;[1 1 1] Random AI spawner
    (`/Engine/EditorBlueprintResources/ActorMacros.Switch Has Authority`
      (:`Authority`
        (`|ExecutionSequence`
          (:`then_0`
            (goto _label :!via `Close`))
          (:`then_1`
            (for _array_element (`self.AIToSpawn`)
              (`self.RespawnAI` _array_element))
            (`|ExecutionSequence`
              (:`then_0`
                (goto _label :!via `Open`))
              (:`then_1`
                (`/Engine/EditorBlueprintResources/StandardMacros.Gate` false :!label _label
                  (:`Exit`
                    (if (`self.SetAIParty?(ex Guards)`)
                      (for _array_element_2 (`self.SpawnedAI`)
                        (`/Game/ActionRPGStarterSystem/AI/BP_AI_Main.SetAIParty` _array_element_2 (`self.SpawnedAI`))))))))))))))

(event `self.Box.OnComponentEndOverlap`
  (params (OverlappedComponent :type "PrimitiveComponent Object Reference") (OtherActor :type "Actor Object Reference") (OtherComp :type "PrimitiveComponent Object Reference") (OtherBodyIndex :type Integer))
  ;[1 1 1] despawn if out of range
  (if (== OtherActor (`GameplayStatics.GetPlayerCharacter` 0))
    (`KismetSystemLibrary.PrintString` "Hello")
    (if (> (`KismetArrayLibrary.Array_Length` (`self.SpawnedAI`)) 0) :!label _label_2
      (`self.K2_DestroyActor` (`self.SpawnedAI`))
      (`KismetSystemLibrary.Delay` 0.1)
      (goto _label_2))))

(event `OnAIDestroyed`
  (params (AIClass :type "/Game/ActionRPGStarterSystem/AI/BP_AI_Main Class Reference") (AIRef :type "/Game/ActionRPGStarterSystem/AI/BP_AI_Main Object Reference"))
  (bind (_isstationaryai _stationarylocation) (`/Game/ActionRPGStarterSystem/AI/BP_AI_Main.IsStationary` AIRef))
  ;[1 1 1] Respawn AI
  (`KismetArrayLibrary.Array_RemoveItem` (`self.SpawnedAI`) AIRef)
  (if (`self.RespawnAI?`)
    (`|SpawnActorFromClass` "/Game/ActionRPGStarterSystem/AI/BP_AIRespawner.BP_AIRespawner_C" (`KismetMathLibrary.MakeTransform` (0.0 0.0 0.0)) "AdjustIfPossibleButAlwaysSpawn" "OverrideRootScale" null AIClass (`self.RespawnAIDelay`) self _isstationaryai _stationarylocation null)))

(event `OnAISpawned`
  (params (AIRef :type "/Game/ActionRPGStarterSystem/AI/BP_AI_Main Object Reference"))
  (`KismetArrayLibrary.Array_AddUnique` (`self.SpawnedAI`) AIRef)
  (`self.ShareAggroKnowledge` AIRef)
  (goto _label))

(event `Respawner_RespawnAI`
  (params (Class :type "/Game/ActionRPGStarterSystem/AI/BP_AI_Main Class Reference") (`IsStationary?` :type Boolean) (StationeryT :type "Transform Structure"))
  ;[1 1 1] Respawn AI
  (`self.RespawnAI` Class `IsStationary?` StationeryT))

(fn `RespawnAI`
  (params (AIClass :type "/Game/ActionRPGStarterSystem/AI/BP_AI_Main Class Reference") (IsStationary :type Boolean) (StationaryT :type "Transform Structure"))
  (returns (SpawnedAI :type "/Game/ActionRPGStarterSystem/AI/BP_AI_Main Object Reference"))
  (if IsStationary
    (bind _returnvalue (`|SpawnActorFromClass` AIClass (`KismetMathLibrary.MakeTransform` (.location StationaryT) (.rotation StationaryT)) "AdjustIfPossibleButAlwaysSpawn" "OverrideRootScale" null (0.0 0.0 0.0) true true self null))
    (`/Engine/EditorBlueprintResources/StandardMacros.IsValid` _returnvalue
      (:`Is Valid`
        (return _returnvalue))
      (:`Is Not Valid`
        _)))
  (bind (_location _found) (`self.TryGetSpawnLocation` 88.0))
  (if _found
    (bind _returnvalue_2 (`|SpawnActorFromClass` AIClass (`KismetMathLibrary.MakeTransform` _location (`KismetMathLibrary.MakeRotator` 0.0 0.0 (`KismetMathLibrary.RandomFloatInRange` 0.0 360.0))) "AdjustIfPossibleButAlwaysSpawn" "OverrideRootScale" null (0.0 0.0 0.0) true true self null))
    (return _returnvalue_2)))

(fn `ShareAggroKnowledge`
  (params (SpawnedAI :type "/Game/ActionRPGStarterSystem/AI/BP_AI_Main Object Reference"))
  (locals (UniqueAggroList :type "Array of Actor Object Reference") (CopyFrom :type "/Game/ActionRPGStarterSystem/AI/BP_AI_Main Object Reference"))
  (for _array_element (`self.SpawnedAI`)
    (if (`/Game/ActionRPGStarterSystem/AI/BP_AI_Main.IsAlive?` _array_element)
      (set `local.CopyFrom` _array_element)
      (`/Game/ActionRPGStarterSystem/AI/BP_AI_Main.AddMultipleAggroTargets` SpawnedAI (`/Game/ActionRPGStarterSystem/AI/BP_AI_Main.GetAggroTargets` (`local.CopyFrom`)))
      (return) ; Exit
    )))

(fn `TryGetSpawnLocation`
  (params (CapsuleHeight :type "Float (double-precision)" :default 88.0) (Raduis :type "Float (double-precision)" :default 15.0))
  (returns (Location :type "Vector Structure") (Found :type Boolean))
  (locals (StartingLoc :type "Vector Structure" :default (0.0 0.0 0.0)) (HitLoc :type "Vector Structure" :default (0.0 0.0 0.0)))
  (bind _startingloc (`local.StartingLoc`))
  ;[1 1 1] Spawn AI, try finding a suitable spot
  (for _ (range 101)
    (bind _output_get (set `local.StartingLoc` (+ (`self.K2_GetActorLocation`) (`KismetMathLibrary.MakeVector` (`KismetMathLibrary.RandomFloatInRange` (* (`self.Radius`) -1.0) (`self.Radius`)) (`KismetMathLibrary.RandomFloatInRange` (* (`self.Radius`) -1.0) (`self.Radius`)) 100.0))))
    (bind (_outhit _returnvalue) (`KismetSystemLibrary.LineTraceSingle` _output_get (+ _output_get (0.0 0.0 -500.0)) "TraceTypeQuery1")) ; Finding the floor
    (if _returnvalue
      (bind _output_get_2 (set `local.HitLoc` (`.ImpactPoint` (`GameplayStatics.BreakHitResult` _outhit))))
      (bind _returnvalue_2 (+ _output_get_2 (`KismetMathLibrary.MakeVector` 0.0 0.0 (+ (`local.CapsuleHeight`) 5.0))))
      (bind (_outhit_2 _returnvalue_3) (`KismetSystemLibrary.CapsuleTraceSingleForObjects` :`Start` _returnvalue_2 :`End` _returnvalue_2 :`Radius` (`local.Raduis`) :`HalfHeight` (- (`local.CapsuleHeight`) 5.0) :`ObjectTypes` (`|MakeArray` "ObjectTypeQuery1" "ObjectTypeQuery2" :!type "EObjectTypeQuery Enum") :`DrawTime` 99.0 :!label _label))
      (if (not _returnvalue_3)
        (return (`.TraceStart` (`GameplayStatics.BreakHitResult` _outhit_2)) true))
      (else
        (set `local.StartingLoc` (+ _startingloc (0.0 0.0 200.0)))
        (bind (_outhit_3 _returnvalue_4) (`KismetSystemLibrary.LineTraceSingle` _startingloc (+ _startingloc (0.0 0.0 -500.0)) "TraceTypeQuery1")) ; Finding the floor
        (if _returnvalue_4
          (set `local.HitLoc` (`.ImpactPoint` (`GameplayStatics.BreakHitResult` _outhit_3)))
          (goto _label)))))
  (return (0.0 0.0 0.0) false))

(fn `UserConstructionScript`
  (`KismetSystemLibrary.DrawDebugSphere` (`self.K2_GetActorLocation`) (`self.Radius`) 12 (struct :`R` 0.152017 :`G` 1.0 :`A` 1.0) 0.1 4.0))