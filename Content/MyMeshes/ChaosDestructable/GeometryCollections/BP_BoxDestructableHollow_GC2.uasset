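; A Chaos field actor that breaks nearby geometry collections when spawned, named for a hollow destructible box.
; On BeginPlay it applies an external cluster strain radial falloff field sized and centered on its Sphere component.
; A radial vector linear velocity field, culled outside the same sphere, pushes fragments outward.
; The actor destroys itself after a delay; construction script and other events are empty.
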(event `self.ReceiveBeginPlay`
  (bind _sphere (`self.Sphere`))
  (bind _returnvalue (`RadialFalloff.SetRadialFalloff` (`self.RadialFalloff`) 100.0 0.0 1.0 0.0 (`SphereComponent.GetScaledSphereRadius` _sphere) (`SceneComponent.K2_GetComponentLocation` _sphere) "Field_FallOff_None"))
  (`FieldSystemComponent.ApplyPhysicsField` (`self.FieldSystem`) true "Field_ExternalClusterStrain" null _returnvalue)
  (`FieldSystemComponent.ApplyPhysicsField` (`self.FieldSystem`) true "Field_LinearVelocity" null (`CullingField.SetCullingField` (`self.CullingField`) _returnvalue (`RadialVector.SetRadialVector` (`self.RadialVector`) 100.0 (`SceneComponent.K2_GetComponentLocation` (`self.Sphere`))) "Field_Culling_Outside"))
  (`KismetSystemLibrary.Delay` 20.0)
  (`self.K2_DestroyActor`))

(fn `UserConstructionScript`)