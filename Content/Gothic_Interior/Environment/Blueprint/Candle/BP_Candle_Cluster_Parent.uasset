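; Parent Blueprint for candle cluster props in the Gothic interior environment, configurable as burning or off, with or without candles in the holders.
; All logic runs in the Construction Script, finding candle meshes and flame particles by component tag to set material and visibility.
; Point lights get a global intensity multiplier when lit and active, otherwise they are hidden.
; A fake bloom sphere is destroyed unless enabled on burning, present candles.
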(fn `UserConstructionScript`
  (bind _candleexist__forholders_ (`self.candleExist?(ForHolders)`))
  (bind _returnvalue (and (`self.candleExist?(ForHolders)`) (select `/Game/Gothic_Interior/Environment/Blueprint/Candle/E_CandleBurnType` (`self.candleBurnType`) :`NewEnumerator0` true)))
  (`SceneComponent.SetVisibility` (`self.DefaultSceneRoot`) true true)
  (for _array_element (`self.GetComponentsByTag` "/Script/Engine.StaticMeshComponent" "Candle")
    (`PrimitiveComponent.SetMaterial` _array_element 0 (select `/Game/Gothic_Interior/Environment/Blueprint/Candle/E_CandleBurnType` (`self.candleBurnType`) :`NewEnumerator0` "/Game/Gothic_Interior/Environment/Asset/Material/MI_Candle_01b.MI_Candle_01b" :`NewEnumerator2` "/Game/Gothic_Interior/Environment/Asset/Material/MI_Candle_Off_01b.MI_Candle_Off_01b" :!type "MaterialInterface Object Reference"))
    (`SceneComponent.SetVisibility` _array_element _candleexist__forholders_ true)
    (`SceneComponent.SetHiddenInGame` _array_element (not _candleexist__forholders_) true))
  (for _array_element_2 (`self.GetComponentsByTag` "/Script/Engine.ParticleSystemComponent" "CandleFire")
    (`SceneComponent.SetVisibility` _array_element_2 _returnvalue true)
    (`SceneComponent.SetHiddenInGame` _array_element_2 (not _returnvalue) true))
  (for _array_element_3 (`self.K2_GetComponentsByClass` "/Script/Engine.PointLightComponent")
    (if (and (`|EnumEquality` (`self.candleBurnType`) "NewEnumerator0") (`self.pointLightActive?`) (`self.candleExist?(ForHolders)`))
      (`LightComponent.SetIntensity` _array_element_3 (* (`LightComponentBase.Intensity` _array_element_3) (`self.globalIntensityMultiplier`)))
      (else
        (`SceneComponent.SetVisibility` _array_element_3 false true)
        (`SceneComponent.SetHiddenInGame` _array_element_3 true true))))
  (if (not (and (`self.fakeBloom?`) (`|EnumEquality` (`self.candleBurnType`) "NewEnumerator0") (`self.candleExist?(ForHolders)`)))
    (`ActorComponent.K2_DestroyComponent` (`self. BloomSphere`))))