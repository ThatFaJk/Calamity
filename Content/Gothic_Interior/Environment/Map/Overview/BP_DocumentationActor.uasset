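; BP_DocumentationActor is an info actor for the Gothic Interior overview map that carries a documentation link and themed text.
; Its construction script copies Link into DocumentLink, then applies the overview theme.
; The theme step finds the BP_Overview_ThemeSystem actor, looks up the ThemeTable row named after its OverviewTheme enum, and colors TextRender with that row's info card text color.
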(fn `ApplyOverviewTheme`
  (bind _returnvalue (`GameplayStatics.GetActorOfClass` "/Game/Gothic_Interior/Environment/Map/Overview/System/BP_Overview_ThemeSystem.BP_Overview_ThemeSystem_C"))
  (bind _returnvalue_2 (`|GetDataTableRow` (`/Game/Gothic_Interior/Environment/Map/Overview/System/BP_Overview_ThemeSystem.Theme Table` _returnvalue) (`KismetStringLibrary.Conv_StringToName` (`|GetEnumeratorNameAsString` (`/Game/Gothic_Interior/Environment/Map/Overview/System/BP_Overview_ThemeSystem.Overview Theme` _returnvalue))))
    (:`then`
      (`TextRenderComponent.SetTextRenderColor` (`self.TextRender`) (`.InfoCardTextColor_29_CD6478004372FDD910EC8CB9B4B53DBE` (break `/Game/Gothic_Interior/Environment/Map/Overview/Structure/S_Overview_Theme` _returnvalue_2))))))

(fn `UserConstructionScript`
  (set `self.DocumentLink` (`self.Link`))
  (`self.ApplyOverviewTheme`))