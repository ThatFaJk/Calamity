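; Documentation text actor for the Gothic Interior overview map whose text color follows the active overview theme.
; On construction, it finds the BP_Overview_ThemeSystem actor and looks up the current theme enum by name in its theme data table.
; The row's info card text color is applied to the TextRender component; BeginPlay and Tick are unused.
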(fn `ApplyOverviewTheme_0`
  (bind _returnvalue (`GameplayStatics.GetActorOfClass` "/Game/Gothic_Interior/Environment/Map/Overview/System/BP_Overview_ThemeSystem.BP_Overview_ThemeSystem_C"))
  (bind _returnvalue_2 (`|GetDataTableRow` (`/Game/Gothic_Interior/Environment/Map/Overview/System/BP_Overview_ThemeSystem.Theme Table` _returnvalue) (`KismetStringLibrary.Conv_StringToName` (`|GetEnumeratorNameAsString` (`/Game/Gothic_Interior/Environment/Map/Overview/System/BP_Overview_ThemeSystem.Overview Theme` _returnvalue))))
    (:`then`
      (`TextRenderComponent.SetTextRenderColor` (`self.TextRender`) (`.InfoCardTextColor_29_CD6478004372FDD910EC8CB9B4B53DBE` (break `/Game/Gothic_Interior/Environment/Map/Overview/Structure/S_Overview_Theme` _returnvalue_2))))))

(fn `UserConstructionScript`
  (`parent.UserConstructionScript`)
  (`self.ApplyOverviewTheme_0`))