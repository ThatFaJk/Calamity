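; Destructible four-box prop that scatters random pickups and can award XP and quest progress when broken.
; SpawnerCondition selects loot on BeginPlay or at zero health from capped damage; interaction or a rolling player's hit also breaks it via the server.
; Breaking swaps the mesh for a Geometry Collection actor and rolls PossibleSpawnPickups by chance, with optional impulse.
; On authority, Destroyed passes its settings to a BP_Respawner when RespawnTime allows.
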(event `self.ReceiveBeginPlay`
  (bind _spawnercondition (`self.SpawnerCondition`))
  ;[0.07812 0.07812 0.07812] Based on the condition we can spawn random items on begin play.
  (set `self.BEGINPlay?` true)
  (`|ExecutionSequence`
    (:`then_0`
      (`/Engine/EditorBlueprintResources/ActorMacros.Switch Has Authority`
        (:`Authority`
          (if (or (`|EnumEquality` _spawnercondition "NewEnumerator0") (`|EnumEquality` _spawnercondition "NewEnumerator3"))
            (`self.ProcessRandomSpawner`)
            (if (`|EnumEquality` (`self.SpawnerCondition`) "NewEnumerator0")
              (`self.K2_DestroyActor`))))))
    (:`then_1`
      (bind _asbp_display_name (cast `/Game/ActionRPGStarterSystem/InventorySystem/JigSaw/Widgets/BP_DisplayName` (`WidgetComponent.GetUserWidgetObject` (`self.Widget`))))
      (`/Game/ActionRPGStarterSystem/InventorySystem/JigSaw/Widgets/BP_DisplayName.UpdateName` _asbp_display_name (`self.SpawnerName`) (`self.SpawnerNameColor`)))))

(event `self.ReceiveAnyDamage`
  (params (Damage :type "Float (single-precision)") (DamageType :type "DamageType Object Reference") (InstigatedBy :type "Controller Object Reference") (DamageCauser :type "Actor Object Reference"))
  (bind _spawnercondition (`self.SpawnerCondition`))
  ;[0.01042 0.01042 0.01042] Spawn items when damaged
  (if (and (or (`|EnumEquality` _spawnercondition "NewEnumerator4") (`|EnumEquality` _spawnercondition "NewEnumerator5")) (> (`self.Health`) 0.0))
    (bind _output_get (set `self.Health` (- (stale _output_get) (`KismetMathLibrary.FClamp` Damage 0.0 (`self.MaxDamagePerHit`)))))
    (if (<= _output_get 0.0)
      (`/Engine/EditorBlueprintResources/StandardMacros.DoOnce` false
        (:`Completed`
          (`self.ServerDestroyComponent`)
          (message `/Game/ActionRPGStarterSystem/Skills/Blueprint/SkillComponent/IT_SkillEffects.Skill_OnTargetExpEarned` DamageCauser self (`self.ExpEarned`) false)
          (set `self.Health` 0.0)
          (`self.ProcessRandomSpawner`)
          (if (`|EnumEquality` (`self.SpawnerCondition`) "NewEnumerator4")
            (`self.CheckQuestOnDestroyObject` DamageCauser)
            (`self.K2_DestroyActor`)))))))

(event `ServerDestroyComponent`
  ;[1 1 1] Destrution when damage taken --> spawns geometry collection actor
  (`ActorComponent.K2_DestroyComponent` (`self.StaticMesh`))
  (`self.ClientDestroyComponentMulticast`))

(event `self.StaticMesh.OnComponentHit`
  (params (HitComponent :type "PrimitiveComponent Object Reference") (OtherActor :type "Actor Object Reference") (OtherComp :type "PrimitiveComponent Object Reference") (NormalImpulse :type "Vector Structure") (Hit :type "HitResult Structure (by ref)"))
  ;[1 1 1] Destroy on rolling
  (if (`self.ActorHasTag` OtherActor "player")
    (bind _rolling_ (message `/Game/MyInterfaces/BP_Rolling_Interface.IsRolling?` OtherActor))
    (if _rolling_
      (bind _inv (message `/Game/ActionRPGStarterSystem/Character/Blueprints/Interfaces/BP_CharacterInventoryInterface.CharacterGetInventoryComponent` OtherActor))
      (`self.ExecuteInteract` OtherActor _inv))))

(event `ClientDestroyComponentMulticast`
  ;[1 1 1] Destrution when damage taken --> spawns geometry collection actor
  (`|SpawnActorFromClass` "/Game/MyMeshes/ChaosDestructable/GeometryCollections/BP_4BoxesDestructableHollow_GC.BP_4BoxesDestructableHollow_GC_C" (`SceneComponent.GetRelativeTransform` (`self.DefaultSceneRoot`)) "Undefined" "OverrideRootScale" null null))

(event `ServerOnRollingDestroy`
  ;[1 1 1] Destroy on rolling
  (`ActorComponent.K2_DestroyComponent` (`self.StaticMesh`))
  (`self.ClientOnRollingDestroyMulti`))

(event `self.ExecuteInteract`
  (params (CharacterRef :type "Actor Object Reference") (Comp :type "/Game/ActionRPGStarterSystem/InventorySystem/Components/BP_InventoryComponent Object Reference"))
  ;[1 1 1] Destroy on rolling
  (if (`self.HasAuthority` CharacterRef)
    (`/Engine/EditorBlueprintResources/StandardMacros.DoOnce` false
      (:`Completed`
        (`self.ServerOnRollingDestroy`)
        (`self.ProcessRandomSpawner`)
        (`self.K2_DestroyActor`)
        (`KismetSystemLibrary.PrintString` "Hello")))
    (else
      (`/Game/ActionRPGStarterSystem/InventorySystem/Components/BP_InventoryComponent.SERVER_RequestInteractWithActor` Comp self))))

(event `ClientOnRollingDestroyMulti`
  ;[1 1 1] Destroy on rolling
  (`|SpawnActorFromClass` "/Game/MyMeshes/ChaosDestructable/GeometryCollections/BP_4BoxesDestructableHollow_GC.BP_4BoxesDestructableHollow_GC_C" (`SceneComponent.GetRelativeTransform` (`self.DefaultSceneRoot`)) "Undefined" "OverrideRootScale" null null))

(event `self.ReceiveDestroyed`
  (`/Engine/EditorBlueprintResources/ActorMacros.Switch Has Authority`
    (:`Authority`
      (if (`self.BEGINPlay?`)
        (`self.Setup Respawner`)))))

(fn `CanBeDamagedByPlayer?`
  (returns (Result :type Boolean))
  (return true))

(fn `CanInteract?`
  (returns (Result :type Boolean) (RequiredDuration :type "Float (double-precision)"))
  (return true (`self.RequiredDurationForInteraction`)))

(fn `CheckQuestOnDestroyObject`
  (params (Causer :type "Actor Object Reference"))
  (`/Engine/EditorBlueprintResources/StandardMacros.IsValid` Causer
    (:`Is Valid`
      (bind _controller (message `/Game/ActionRPGStarterSystem/Character/Blueprints/Interfaces/BP_CharacterInventoryInterface.CharacterGetControllerRef` Causer))
      (`/Engine/EditorBlueprintResources/StandardMacros.IsValid` _controller
        (:`Is Valid`
          (bind _comp (message `/Game/ActionRPGStarterSystem/Character/Blueprints/Interfaces/BP_QuestInterface.GetQuestComponent` _controller))
          (`/Game/ActionRPGStarterSystem/QuestSystem/BP_PlayerQuestComponent.QuestTrack_OnActorKilled` _comp self))))))

(fn `GetAcceptableDistance`
  (returns (Distance :type "Float (double-precision)"))
  (return 100.0))

(fn `GetActorName`
  (returns (PlayerName :type String))
  (return ""))

(fn `GetAIBehavior`
  (returns (Behavior :type "/Game/ActionRPGStarterSystem/AI/Data/E_AIBehaviorType Enum"))
  (return "NewEnumerator3"))

(fn `GetAIHostility`
  (returns (Result :type "/Game/ActionRPGStarterSystem/AI/Data/E_AIHostilityType Enum"))
  (return "NewEnumerator3"))

(fn `GetBountyExp`
  (returns (Exp :type "Float (double-precision)"))
  (return (`self.ExpEarned`)))

(fn `GetOutlineColor`
  (returns (Color :type "LinearColor Structure"))
  (return (struct :`G` 0.068932 :`B` 1.0 :`A` 1.0)))

(fn `OnBeginInteract`
  (returns (Result :type Boolean))
  (`|ExecutionSequence`
    (:`then_0`
      (if (> (`self.RequiredDurationForInteraction`) 0.0)
        (bind _asbp_display_name (cast `/Game/ActionRPGStarterSystem/InventorySystem/JigSaw/Widgets/BP_DisplayName` (`WidgetComponent.GetUserWidgetObject` (`self.Widget`))))
        (`/Game/ActionRPGStarterSystem/InventorySystem/JigSaw/Widgets/BP_DisplayName.SetProgressbarAnim` _asbp_display_name (`self.RequiredDurationForInteraction`))))
    (:`then_1`
      (return true))))

(fn `OnEndInteract`
  (returns (Result :type Boolean))
  (`|ExecutionSequence`
    (:`then_0`
      (if (> (`self.RequiredDurationForInteraction`) 0.0)
        (bind _asbp_display_name (cast `/Game/ActionRPGStarterSystem/InventorySystem/JigSaw/Widgets/BP_DisplayName` (`WidgetComponent.GetUserWidgetObject` (`self.Widget`))))
        (`/Game/ActionRPGStarterSystem/InventorySystem/JigSaw/Widgets/BP_DisplayName.StopProgressbarAnim` _asbp_display_name)))
    (:`then_1`
      (return true))))

(fn `ProcessRandomSpawner`
  (locals (NumOfspawns :type Integer) (SpawnedActor :type "Actor Object Reference"))
  (bind _returnvalue (`KismetMathLibrary.RandomFloatInRange` 0.0 360.0))
  (bind _xyinpulse (`self.XYInpulse`))
  (bind _maxrandomspawndistance (`self.MaxRandomSpawnDistance`))
  (bind _returnvalue_2 (* _xyinpulse -1.0))
  (bind _returnvalue_3 (+ (`self.K2_GetActorLocation`) (`KismetMathLibrary.MakeVector` (`KismetMathLibrary.RandomFloatInRange` (* _maxrandomspawndistance -1.0) _maxrandomspawndistance) (`KismetMathLibrary.RandomFloatInRange` (* _maxrandomspawndistance -1.0) _maxrandomspawndistance) 50.0)))
  (for _array_element (`self.PossibleSpawnPickups`)
    (bind (_blueprinttospawn _mincount _maxcount _spawnchance _rolltimes) (break `/Game/ActionRPGStarterSystem/OtherBlueprints/RandomSpawner/Structs/JigSpawnInfo` _array_element))
    (for _ (range _rolltimes)
      (if (<= (`KismetMathLibrary.RandomFloatInRange` 1.0 100.0) _spawnchance)
        (`/Engine/EditorBlueprintResources/StandardMacros.IncrementInt` (`local.NumOfspawns`)
          (:`  `
            (bind _asbp_main_pickup_class (castclass `/Game/ActionRPGStarterSystem/InventorySystem/JigSaw/PickupSystem/BP_MainPickupClass` _blueprinttospawn)
              (:`then`
                (bind _returnvalue_4 (`|SpawnActorFromClass` :`Class` _asbp_main_pickup_class :`SpawnTransform` (`KismetMathLibrary.MakeTransform` _returnvalue_3 (`KismetMathLibrary.MakeRotator` 0.0 0.0 _returnvalue)) :`CollisionHandlingOverride` "AdjustIfPossibleButAlwaysSpawn" :`TransformScaleMethod` "OverrideRootScale" :`NewCount` (`KismetMathLibrary.RandomIntegerInRange` _mincount _maxcount) :`Instigator` null))
                (set `local.SpawnedActor` _returnvalue_4))
              (:`CastFailed`
                (bind _returnvalue_5 (`|SpawnActorFromClass` _blueprinttospawn (`KismetMathLibrary.MakeTransform` _returnvalue_3 (`KismetMathLibrary.MakeRotator` 0.0 0.0 _returnvalue)) "AdjustIfPossibleButAlwaysSpawn" "OverrideRootScale" null null))
                (set `local.SpawnedActor` _returnvalue_5)))
            (`|ExecutionSequence`
              (:`then_0`
                (if (`self.ApplyInpulse?`)
                  (bind _asprimitive_component (cast `PrimitiveComponent` (`Actor.RootComponent` (`local.SpawnedActor`))))
                  (`PrimitiveComponent.AddImpulse` _asprimitive_component (`KismetMathLibrary.MakeVector` (`KismetMathLibrary.RandomFloatInRange` _returnvalue_2 _xyinpulse) (`KismetMathLibrary.RandomFloatInRange` _returnvalue_2 _xyinpulse) (`self.ZInpulse`)) "None" false)))
              (:`then_1`
                (if (== (`local.NumOfspawns`) (`self.MaxItemsToSpawn`))
                  (return))))))))))

(fn `SetHostility`
  (params (NewHostility :type "/Game/ActionRPGStarterSystem/AI/Data/E_AIHostilityType Enum" :default "NewEnumerator3"))
  (returns (Result :type Boolean))
  (return false))

(fn `SetHostilityColor`
  (params (IsHostile :type Boolean) (`IsParty?` :type Boolean) (`IsGuild?` :type Boolean))
  (returns (Result :type Boolean))
  (return false))

(fn `SetOutlineEnabled`
  (params (Enabled :type Boolean) (InteractKey :type "Key Structure") (CalledFrom :type "Actor Object Reference"))
  (returns (`Enabled?` :type Boolean))
  (bind _spawnercondition (`self.SpawnerCondition`))
  (bind _returnvalue (== InteractKey (`self.NoneKey`)))
  (bind _output_get (set `self.OutlineOn` Enabled))
  (set `/Game/ActionRPGStarterSystem/InventorySystem/JigSaw/PickupSystem/BP_NameVisibility.OutlineOn` _output_get (`self.BP_NameVisibility`))
  (`|ExecutionSequence`
    (:`then_0`
      (if (or (`|EnumEquality` _spawnercondition "NewEnumerator1") (`|EnumEquality` _spawnercondition "NewEnumerator2"))
        (if (not _returnvalue)
          (bind _asbp_display_name (cast `/Game/ActionRPGStarterSystem/InventorySystem/JigSaw/Widgets/BP_DisplayName` (`WidgetComponent.GetUserWidgetObject` (`self.Widget`))))
          (`/Game/ActionRPGStarterSystem/InventorySystem/JigSaw/Widgets/BP_DisplayName.SetInteractKey` _asbp_display_name (`KismetInputLibrary.Key_GetDisplayName` InteractKey) (or _returnvalue (not _output_get))))))
    (:`then_1`
      (return _output_get))))

(fn `Setup Respawner`
  (locals (Time :type "Float (double-precision)" :default 0.0))
  (bind (_origin _boxextent) (`self.GetActorBounds` true))
  (bind (_respawntime_x _respawntime_y) (`KismetMathLibrary.BreakVector2D` (`self.RespawnTime`)))
  (if (> _respawntime_y 0.0)
    (`|SpawnActorFromClass` "/Game/ActionRPGStarterSystem/OtherBlueprints/RandomSpawner/BP_Respawner.BP_Respawner_C" (`KismetMathLibrary.MakeTransform` (0.0 0.0 0.0)) "AdjustIfPossibleButAlwaysSpawn" "OverrideRootScale" null (`GameplayStatics.GetObjectClass` self) (`self.RespawnTime`) (`SceneComponent.K2_GetComponentToWorld` (`self.RootComponent`)) (`self.PossibleSpawnPickups`) (`self.SpawnerCondition`) (`self.MaxHealth`) (`self.MaxDamagePerHit`) (`self.ApplyInpulse?`) (`self.XYInpulse`) (`self.ZInpulse`) (`self.MaxItemsToSpawn`) (`self.RequiredDurationForInteraction`) (`self.ExpEarned`) (`self.MaxRandomSpawnDistance`) (`self.SpawnerNameColor`) (`self.SpawnerName`) (`self.ShowNameWidget?`) _origin _boxextent null)))

(fn `UserConstructionScript`
  (set `self.MaxHealth` (`self.Health`))
  (if (`self.ShowNameWidget?`)
    (set `/Game/ActionRPGStarterSystem/InventorySystem/JigSaw/PickupSystem/BP_NameVisibility.Widget` (`self.Widget`) (`self.BP_NameVisibility`))
    (else
      (`SceneComponent.SetVisibility` (`self.Widget`) false false))))