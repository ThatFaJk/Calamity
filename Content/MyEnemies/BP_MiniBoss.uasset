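; BP_MiniBoss is a mini-boss enemy Blueprint that toggles a boss health display for nearby local players.
; Overlaps on TriggerBossHealthBar filter for Player-tagged pawns with a valid, locally controlled controller.
; Entering calls ShowBossHealth with that player controller and leaving calls RemoveBossHealth, so only locally controlled players trigger the display.
; The construction script only calls its parent.
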(event `self.TriggerBossHealthBar.OnComponentBeginOverlap`
  (params (OverlappedComponent :type "PrimitiveComponent Object Reference") (OtherActor :type "Actor Object Reference") (OtherComp :type "PrimitiveComponent Object Reference") (OtherBodyIndex :type Integer) (bFromSweep :type Boolean) (SweepResult :type "HitResult Structure (by ref)"))
  (if (`self.ActorHasTag` OtherActor "Player")
    (bind _aspawn (cast `Pawn` OtherActor))
    (bind _returnvalue (`self.GetController` _aspawn))
    (`/Engine/EditorBlueprintResources/StandardMacros.IsValid` _returnvalue
      (:`Is Valid`
        (if (`Controller.IsLocalController` _returnvalue)
          (bind _asplayer_controller (cast `PlayerController` _returnvalue))
          (`self.ShowBossHealth` _asplayer_controller))))))

(event `self.TriggerBossHealthBar.OnComponentEndOverlap`
  (params (OverlappedComponent :type "PrimitiveComponent Object Reference") (OtherActor :type "Actor Object Reference") (OtherComp :type "PrimitiveComponent Object Reference") (OtherBodyIndex :type Integer))
  (if (`self.ActorHasTag` OtherActor "Player")
    (bind _aspawn (cast `Pawn` OtherActor))
    (bind _returnvalue (`self.GetController` _aspawn))
    (`/Engine/EditorBlueprintResources/StandardMacros.IsValid` _returnvalue
      (:`Is Valid`
        (if (`Controller.IsLocalController` _returnvalue)
          (`self.RemoveBossHealth` null))))))

(fn `UserConstructionScript`
  (`parent.UserConstructionScript`))