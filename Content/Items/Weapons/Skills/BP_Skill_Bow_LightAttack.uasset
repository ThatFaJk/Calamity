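; Bow light attack skill actor that acts as an arrow, damaging a single enemy.
; On server-side sphere overlap it damages living, damageable hostiles with effects, triggers the owner's skill sound and destroys itself; Hit also destroys it.
; When locked on, construction rotates it toward the skill target, with a debug print flagging this as needing a fix.
; A helper, uncalled here, derives aim direction from a camera trace.
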(event `self.ReceiveBeginPlay`
  (`parent.ReceiveBeginPlay`))

(event `self.Sphere.OnComponentBeginOverlap`
  (params (OverlappedComponent :type "PrimitiveComponent Object Reference") (OtherActor :type "Actor Object Reference") (OtherComp :type "PrimitiveComponent Object Reference") (OtherBodyIndex :type Integer) (bFromSweep :type Boolean) (SweepResult :type "HitResult Structure (by ref)"))
  (if (!= OtherActor (`self.PawnOwner`))
    (`/Engine/EditorBlueprintResources/ActorMacros.Switch Has Authority`
      (:`Authority`
        (if (and (`Actor.bCanBeDamaged` OtherActor) (`self.IsTargetHostile` OtherActor) (`self.IsTargetAlive?` OtherActor))
          (`self.DamageSingleEnemyByRef` OtherActor (`self.SkillDamage`) (`self.DamageType`) true)
          (`|ExecutionSequence`
            (:`then_0`
              (bind _pawnowner (`self.PawnOwner`)
                (:`then`
                  (message `/Game/ActionRPGStarterSystem/Skills/Blueprint/SkillComponent/IT_SkillEffects.Skill_MCSound` _pawnowner null (`self.K2_GetActorLocation`)))
                (:`else`)))
            (:`then_1`
              (`self.K2_DestroyActor`))))))))

(event `self.ReceiveHit`
  (params (MyComp :type "PrimitiveComponent Object Reference") (Other :type "Actor Object Reference") (OtherComp :type "PrimitiveComponent Object Reference") (bSelfMoved :type Boolean) (HitLocation :type "Vector Structure") (HitNormal :type "Vector Structure") (NormalImpulse :type "Vector Structure") (Hit :type "HitResult Structure (by ref)"))
  (`self.K2_DestroyActor`))

(fn `Calculate Location For Arrow`
  (returns (NewDirection :type "Vector Structure"))
  (bind _returnvalue (`self.GetComponentByClass` (`self.PawnOwner`) "/Script/Engine.CameraComponent"))
  (bind _returnvalue_2 (`SceneComponent.K2_GetComponentLocation` _returnvalue))
  (bind (_outhit _returnvalue_3) (`KismetSystemLibrary.LineTraceSingle` :`Start` _returnvalue_2 :`End` (+ _returnvalue_2 (* (`SceneComponent.GetForwardVector` _returnvalue) 10000.0)) :`TraceChannel` "TraceTypeQuery1" :`DrawDebugType` "ForDuration"))
  (bind (_bblockinghit _binitialoverlap _time _distance _location _impactpoint _normal _impactnormal _physmat _hitactor _hitcomponent _hitbonename _bonename _hititem _elementindex _faceindex _tracestart _traceend) (`GameplayStatics.BreakHitResult` _outhit))
  (return (`KismetMathLibrary.GetDirectionUnitVector` (`self.K2_GetActorLocation`) (`KismetMathLibrary.SelectVector` _location _traceend _returnvalue_3))))

(fn `UserConstructionScript`
  (`parent.UserConstructionScript`)
  (`/Engine/EditorBlueprintResources/StandardMacros.IsValid` (`self.PawnOwner`)
    (:`Is Valid`
      (if (`self.IsLockedOnForArrow`)
        (`KismetSystemLibrary.PrintString` "IT SHOULD WORK \nSTILL NEEDS FIX \n")
        (`self.K2_SetActorRotation` (`KismetMathLibrary.FindLookAtRotation` (`self.K2_GetActorLocation`) (`self.K2_GetActorLocation` (`self.SkillTarget`))) true)))))