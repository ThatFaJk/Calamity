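; Bus station light Blueprint that simulates a faulty, flickering lamp by driving a SpotLight's intensity.
; TurnOn starts a delay loop of short random intensity flickers, counted up to a burst, followed by full brightness for a random hold.
; TurnOff clears IsOn and zeroes the intensity, but the loop checks the flag only after each hold, so an ongoing burst can briefly relight the lamp.
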(event `TurnOn`
  (bind _output_get (set `self.IsOn` true))
  (if _output_get
    (`LightComponent.SetIntensity` (`self.SpotLight`) (`KismetMathLibrary.RandomFloatInRange` 0.0 5000.0) :!label _label)
    (bind _result (`/Engine/EditorBlueprintResources/StandardMacros.IncrementInt` (`self.count`))
      (:`  `
        (if (>= _result 5)
          (`LightComponent.SetIntensity` (`self.SpotLight`) 5000.0)
          (`KismetSystemLibrary.Delay` (`KismetMathLibrary.RandomFloatInRange` 1.0 5.0))
          (set `self.count` 0)
          (if (`self.IsOn`)
            (`KismetSystemLibrary.Delay` (`KismetMathLibrary.RandomFloatInRange` 0.0 0.2) :!label _label_2)
            (goto _label)
            (else
              (`LightComponent.SetIntensity` (`self.SpotLight`) 0.0)))
          (else
            (goto _label_2)))))))

(event `TurnOff`
  (set `self.IsOn` false)
  (`LightComponent.SetIntensity` (`self.SpotLight`) 0.0))

(fn `UserConstructionScript`)